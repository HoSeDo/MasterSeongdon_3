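; Sandbox pistol weapon Blueprint that fires hitscan shots and calls Fire two seconds after BeginPlay.
; SandboxFire checks CanFire and ammo, then plays a shot sound, line-traces along the FirePoint forward vector and updates ammo.
; Each shot also starts a fire-delay timer derived from the rate of fire.
; A failed ammo check triggers a reload with its own sound.
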(event `self.ReceiveBeginPlay`
  (`KismetSystemLibrary.Delay` 2.0)
  (`self.Fire`))

(event `self.SandboxFire`
  (if (`self.CanFire`)
    (`self.CheckAmmo`)
    (if true
      (`|ExecutionSequence`
        (:`then_0`
          (`self.PlaySound` "/Game/Audio/Explosion02.Explosion02")
          (`self.LinetraceOneShot` (`SceneComponent.GetForwardVector` (`self.FirePoint`)))
          (`self.UpdateAmmo`))
        (:`then_1`
          (bind _returnvalue (`KismetSystemLibrary.K2_SetTimer` null "" (/ 1.0 (`self.RoF`))))
          (set `self.TimerFireDelay` _returnvalue)))
      (else
        (`self.Reload`)
        (`self.PlaySound` "/Game/Audio/Fire01.Fire01")))))

(fn `UserConstructionScript`)