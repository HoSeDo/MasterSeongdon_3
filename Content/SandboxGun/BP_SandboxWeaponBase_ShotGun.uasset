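; Shotgun weapon Blueprint, apparently built on a shared sandbox weapon base, that fires a spread of hitscan pellets.
; SandboxFire, gated by CanFire, plays a blast sound and loops random-cone line traces, updating ammo per pellet.
; It then clears CanFire and starts a rate-of-fire timer that names no function.
; The branch after CheckAmmo is constant true, leaving reload unreachable; BeginPlay calls Fire after a delay.
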(event `self.ReceiveBeginPlay`
  (`KismetSystemLibrary.Delay` 2.0)
  (`self.Fire`))

(event `self.SandboxFire`
  (if (`self.CanFire`)
    (`KismetSystemLibrary.PrintString` (`KismetStringLibrary.Conv_IntToString` (`self.CurrentAmmo`)))
    (`self.CheckAmmo`)
    (if true
      (`|ExecutionSequence`
        (:`then_0`
          (`self.PlaySound` "/Game/Audio/Explosion02.Explosion02")
          (for _ (range 1 6)
            (`self.LinetraceOneShot` (`KismetMathLibrary.RandomUnitVectorInConeInDegrees` (`SceneComponent.GetForwardVector` (`self.FirePoint`)) 20.0))
            (`self.UpdateAmmo`)))
        (:`then_1`
          (bind _returnvalue (`KismetSystemLibrary.K2_SetTimer` null "" (/ 1.0 (`self.RoF`))))
          (set `self.TimerFireDelay` _returnvalue)
          (set `self.CanFire` false)))
      (else
        (`self.Reload`)
        (`self.PlaySound` "/Game/Audio/Light01.Light01")))))

(fn `UserConstructionScript`)